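; LevelMap builds a linear chain of rooms at runtime when play begins.
; Starting from StartRoom, a fixed-count loop spawns FbxScene_Room actors at the origin, then positions each at door 1 of the previous room.
; Each new room becomes the next attachment point and has its doors 1 and 2 set inactive.
; Placement and door logic are delegated to the room actor, and Tick is unused.
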(event `self.ReceiveBeginPlay`
  (set `self.LastRoom` (`self.StartRoom`))
  (for _ (range 6)
    (bind _returnvalue (`|SpawnActorFromClass` "/Game/Meshes/Level/FbxScene_Room.FbxScene_Room_C" (`KismetMathLibrary.Conv_VectorToTransform` (`KismetMathLibrary.MakeVector` 0.0)) "AlwaysSpawn" "OverrideRootScale"))
    (`/Game/Meshes/Level/FbxScene_Room.PositionAtDoor` _returnvalue (`self.LastRoom`) 1)
    (bind _output_get (set `self.LastRoom` _returnvalue))
    (`/Game/Meshes/Level/FbxScene_Room.SetDoorActive` _output_get 1 false)
    (`/Game/Meshes/Level/FbxScene_Room.SetDoorActive` _output_get 2 false)))